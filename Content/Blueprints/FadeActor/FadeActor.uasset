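; Actor that fades its static mesh in and out through a "Fade" material scalar parameter.
; The construction script caches the original materials and builds dynamic instances from FadeMaterials.
; Fadein swaps in those instances and plays a timeline that drives the parameter, while FadeOut only reverses that timeline.
; When the timeline finishes with Fade at 1, the original materials are restored.
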(event EventFadein
  (CallFunction|SetDynamicMaterial)
  (bind _fade (Timeline|FadeTimeLine PlayFromStart)
    (:Update
      (Rendering|Material|SetScalarParameterValueonMaterials (Variables|Default|GetStaticMesh) "Fade" _fade))
    (:Finished
      (if (== _fade 1.0)
        ;[1 1 1] FadeOut 结果
        (CallFunction|SetOriginalMaterial)))))

(event EventFadeOut
  (bind _fade (Timeline|FadeTimeLine Reverse)
    (:Update
      (Rendering|Material|SetScalarParameterValueonMaterials (Variables|Default|GetStaticMesh) "Fade" _fade))
    (:Finished
      (if (== _fade 1.0)
        ;[1 1 1] FadeOut 结果
        (CallFunction|SetOriginalMaterial)))))

(fn ConstructionScript
  (Variables|Default|SetOringinal%20Material (Rendering|Material|GetMaterials (Variables|Default|GetStaticMesh)))
  (for _array_element (Variables|Default|GetFadeMaterials)
    (bind _returnvalue (Rendering|Material|CreateDynamicMaterialInstance _array_element "None" "None" :!class /Script/Engine.KismetMaterialLibrary))
    (Utilities|Array|AddUnique (Variables|Default|GetDynamicFadeMaterial) _returnvalue)))

(fn SetDynamicMaterial
  (for (_array_element _array_index) (Variables|Default|GetDynamicFadeMaterial)
    (Rendering|Material|SetMaterial (Variables|Default|GetStaticMesh) _array_index _array_element)))

(fn SetOriginalMaterial
  (for (_array_element _array_index) (Variables|Default|GetOringinal%20Material)
    (Rendering|Material|SetMaterial (Variables|Default|GetStaticMesh) _array_index _array_element)))