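; BP_EnemyBase is a base enemy Blueprint that sets up character attributes, dissolve effects and attack facing.
; On BeginPlay it initializes its ability system component's attributes for the Ranger class at its own level.
; Two timelines drive the Dissolve material parameter on the body mesh and weapon separately.
; An interface event updates the FacingTarget motion warp location from a supplied target.
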(event EventBeginPlay
  (|CallParentFunction)
  (Class|AuraBlueprintFunctionLibrary|SetAttributeInfo "Ranger" self (Variables|Default|GetAbilityComponent) (Math|Conversions|ToFloat(Integer) (Variables|Default|GetLevel))))

(event EventWrapActorInterface
  (params (Target :type Vector :default "0, 0, 0"))
  (Class|MotionWarpingComponent|AddorUpdateWarpTargetfromLocation (Variables|组件|GetMotionWarping) "FacingTarget" Target))

(event EventTimeLineSetMeshMaterial
  (bind _新建轨道_0 (Timeline|时间轴_0 Play)
    (:Update
      (Rendering|Material|SetScalarParameterValueonMaterials (Variables|Character|GetMesh) "Dissolve" _新建轨道_0))))

(event EventTimeLineSetWeaponMaterial
  (bind _新建轨道_0 (Timeline|时间轴 Play)
    (:Update
      (Rendering|Material|SetScalarParameterValueonMaterials (Variables|Default|GetWeapon) "Dissolve" _新建轨道_0))))

(fn ConstructionScript
  (|CallParentFunction))