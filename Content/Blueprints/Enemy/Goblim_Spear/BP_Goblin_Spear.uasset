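; Spear goblin enemy Blueprint that sets up its attributes and drives dissolve effects on its body and weapon.
; On BeginPlay it passes the Ranger character class and its level to SetAttributeInfo on its ability system component.
; Two material events each play a timeline that writes the "Dissolve" scalar parameter, one on the mesh materials and one on the weapon materials.
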(event EventBeginPlay
  (Class|AuraBlueprintFunctionLibrary|SetAttributeInfo "Ranger" self (Variables|Default|GetAbilityComponent) (Math|Conversions|ToFloat(Integer) (Variables|Default|GetLevel))))

(event EventTimeLineSetMeshMaterial
  (bind _新建轨道_0 (Timeline|MeshDissolveTL Play)
    (:Update
      (Rendering|Material|SetScalarParameterValueonMaterials (Variables|Character|GetMesh) "Dissolve" _新建轨道_0))))

(event EventTimeLineSetWeaponMaterial
  (bind _新建轨道_0 (Timeline|WeaponDissolveTL Play)
    (:Update
      (Rendering|Material|SetScalarParameterValueonMaterials (Variables|Default|GetWeapon) "Dissolve" _新建轨道_0))))

(fn ConstructionScript)