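; GA_RangeAttack is a Gameplay Ability for a ranged attack that fires a fire bolt at the avatar's target actor.
; It fetches the target through avatar messages, passes its location back to the avatar, and plays a random tagged attack montage.
; The montage's gameplay event tag triggers SpawnFireBolt at the target's current location, then the ability ends.
; An invalid target ends the ability immediately.
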(event Ability|EventActivateAbility
  (Variables|Default|SetAvator (Ability|GetAvatarActorfromActorInfo))
  (bind _returnvalue (Class|EnemyInterface|GetTargetActor(Message) (Variables|Default|GetAvator)))
  (Variables|Default|SetTarget _returnvalue)
  (if (Utilities|IsValid _returnvalue)
    (Class|ICombatInterface|WrapActorInterface(Message) (Variables|Default|GetAvator) (Transformation|GetActorLocation (Variables|Default|GetTarget)))
    (bind _returnvalue_2 (Class|ICombatInterface|GetAttackMontage(Message) (Variables|Default|GetAvator)))
    (Variables|Default|SetTagMontage (.OutItem (Utilities|Array|Random _returnvalue_2)))
    (|PlayMontageandWaitProxy "None" (.attackmontage (Variables|Default|GetTagMontage)) 1.0 "Begin" true 1.0 0.0 false
      (:then
        (Ability|Async|WaitGameplayEventToActor (Variables|Default|GetAvator) (.tag (Variables|Default|GetTagMontage))
          (:EventReceived
            (Class|ProjectileSpell|SpawnFireBolt (Transformation|GetActorLocation (Variables|Default|GetTarget)))
            (Ability|EndAbility)))))
    (else
      (Ability|EndAbility))))

(event Ability|EventOnEndAbility
  (params (bWasCancelled :type Boolean)))