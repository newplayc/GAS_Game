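; Channeled lightning gameplay ability that locks the caster in place and links a beam to the target and nearby enemies.
; After target data and a montage event, a trace from the weapon picks the hit actor and starts looping cues.
; Looping timers commit cost and apply effects, with damage and chain targeting done on the server.
; Input release on the server or a failed cost commit clears timers and cues, restores walking and commits cooldown.
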(event Custom|Cost%20CoolDown
  (bind _returnvalue (Ability|CommitAbilityCost false))
  (if _returnvalue
    (if (Utilities|DoesObjectImplementInterface (Variables|Default|GetHit%20Actor) "/Script/GAS_Game.ICombatInterface")
      (Ability|HasAuthority
        (:True
          (bind _hit_actor (Variables|Default|GetHit%20Actor)
            (:then
              (bind _returnvalue_2 (Class|AuraGameplayDamageAbility|MakeDefaultEffectParams _hit_actor))
              (Class|AuraBlueprintFunctionLibrary|ApplyEffectParams _returnvalue_2))
            (:else)))))
    (else
      (CallFunction|StopAbility))))

(event Custom|Cause%20Additional%20Damage
  ;[1 0.2661 0.6677] 链接其他敌人
  (for _array_element (Variables|Default|GetNear%20Enemies)
    (bind _output_get (Variables|Default|SetArray%20Element _array_element))
    (Utilities|IsValid _output_get
      (:Is%20Valid
        (bind _returnvalue (Class|AuraGameplayDamageAbility|MakeDefaultEffectParams (Variables|Default|GetArray%20Element)))
        (Class|AuraBlueprintFunctionLibrary|ApplyEffectParams _returnvalue)))))

(event Ability|EventActivateAbility
  (bind _damagefrequency (Variables|Default|GetDamageFrequency))
  (bind _damagefrequency_2 (Variables|Default|GetDamageFrequency))
  (if (Utilities|DoesObjectImplementInterface (Ability|GetAvatarActorfromActorInfo) "/Script/GAS_Game.ICombatInterface")
    (Class|LightningLinkAbility|SetParams)
    (bind _datahandle (|TagetData)
      (:TargetData
        (Variables|Default|SetHitLocation (.Location (Collision|BreakHitResult (Ability|TargetData|GetHitResultfromTargetData _datahandle))))
        (Utilities|FlowControl|Sequence
          (:then_0
            (Ability|Tasks|WaitInputRelease true
              (:OnRelease
                (Ability|HasAuthority
                  (:True
                    (CallFunction|StopAbility))
                  (:False
                    (Development|PrintString "Hello"))))))
          (:then_1
            (Class|ICombatInterface|WrapActorInterface(Message) (Ability|GetAvatarActorfromActorInfo) (Variables|Default|GetHitLocation))
            (GameplayCue|ExecuteGameplayCue :GameplayCueTag "(TagName=\"GameplayCue.LightningLinkBurst\")")
            (|PlayMontageandWaitProxy "None" "/Game/Assets/Characters/Aura/Animations/Abilities/AM_Cast_Electrocute.AM_Cast_Electrocute" 1.0 "None" true 1.0 0.0 false
              (:then
                (Ability|Async|WaitGameplayEventToActor (Ability|GetAvatarActorfromActorInfo) "(TagName=\"Event.Montage.LightningLink\")" true
                  (:EventReceived
                    (Utilities|PreCondition)
                    (GameplayCue|AddGameplayCueOnActor(Looping) (Ability|GetAvatarActorfromActorInfo) "(TagName=\"GameplayCue.LightningLinkLoop\")" (Ability|GameplayCue|MakeGameplayCueParameters :Location (Variables|Default|GetHitLocation) :Instigator (Variables|Default|GetNowCharacter) :TargetAttachComponent (Variables|Default|GetWeaponMesh)))
                    (bind _returnvalue (Utilities|Time|SetTimerbyEvent (delegate Custom|Cost%20CoolDown) _damagefrequency true false (Utilities|获取相反数 _damagefrequency)))
                    (Variables|Default|SetCost%20Handle _returnvalue)
                    (if (Utilities|DoesObjectImplementInterface (Variables|Default|GetHit%20Actor) "/Script/GAS_Game.ICombatInterface")
                      ;[1 0.2661 0.6677] 链接其他敌人
                      (Ability|HasAuthority
                        (:True
                          (bind _nearenemies (Class|LightningLinkAbility|GetNearEnemys (Variables|Default|GetHit%20Actor)))
                          (bind _output_get (Variables|Default|SetNear%20Enemies _nearenemies))
                          (for _array_element _output_get
                            (Variables|Default|SetArray%20Element _array_element)
                            (bind _array_element_2 (Variables|Default|GetArray%20Element)
                              (:then
                                (GameplayCue|AddGameplayCueOnActor(Looping) _array_element_2 "(TagName=\"GameplayCue.LightningLinkEnemyLoop\")" (Ability|GameplayCue|MakeGameplayCueParameters :Location (Transformation|GetActorLocation (Variables|Default|GetHit%20Actor)) :TargetAttachComponent (Variables|/Script/Engine.Actor|GetRootComponent (Variables|Default|GetArray%20Element)))))
                              (:else)))
                          (bind _returnvalue_2 (Utilities|Time|SetTimerbyEvent (delegate Custom|Cause%20Additional%20Damage) _damagefrequency_2 true false (Utilities|获取相反数 _damagefrequency_2)))
                          (Variables|Default|SetAdditional%20Damage%20Handle _returnvalue_2))))))))))))
    (else
      (Ability|EndAbility))))

(fn LinkAdditional
  ;[1 0.2661 0.6677] 链接其他敌人
  (Class|AuraGameplayDamageAbility|CauseDamage (Variables|Default|GetHit%20Actor))
  (bind _nearenemies (Class|LightningLinkAbility|GetNearEnemys (Variables|Default|GetHit%20Actor)))
  (bind _output_get (Variables|Default|SetNear%20Enemies _nearenemies))
  (for _array_element _output_get
    (bind _output_get_2 (Variables|Default|SetArray%20Element _array_element))
    (GameplayCue|AddGameplayCueOnActor(Looping) _output_get_2 "(TagName=\"GameplayCue.LightningLinkEnemyLoop\")" (Ability|GameplayCue|MakeGameplayCueParameters :Location (Transformation|GetActorLocation (Variables|Default|GetHit%20Actor)) :TargetAttachComponent (Variables|/Script/Engine.Actor|GetRootComponent (Variables|Default|GetArray%20Element)))))
  (bind _returnvalue (Utilities|Time|SetTimerbyEvent 0 (Variables|Default|GetDamageFrequency) true))
  (Variables|Default|SetAdditional%20Damage%20Handle _returnvalue))

(fn StopAbility
  ;[1 0 0.02983] 松开
  (Pawn|Components|CharacterMovement|SetMovementMode (Variables|/Script/Engine.Character|GetCharacterMovement (Variables|Default|GetNowCharacter)) "MOVE_Walking" 0)
  (Utilities|Time|ClearandInvalidateTimerbyHandle (Variables|Default|GetAdditional%20Damage%20Handle))
  (Utilities|Time|ClearandInvalidateTimerbyHandle (Variables|Default|GetCost%20Handle))
  (Class|PlayerInterface|SetElectricLink(Message) (Variables|Default|GetNowCharacter) false)
  (GameplayCue|RemoveGameplayCue "(TagName=\"GameplayCue.LightningLinkLoop\")")
  (if (Utilities|DoesObjectImplementInterface (Variables|Default|GetHit%20Actor) "/Script/GAS_Game.ICombatInterface")
    (for _array_element (Variables|Default|GetNear%20Enemies)
      (GameplayCue|RemoveGameplayCueOnActor(Looping) _array_element "(TagName=\"GameplayCue.LightningLinkEnemyLoop\")" (Ability|GameplayCue|MakeGameplayCueParameters 0.0))))
  (Ability|CommitAbilityCooldown false)
  (Ability|EndAbility))