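; Fireball Gameplay Ability that casts a projectile at a targeted location, reusing the FireBolt montage, event tag and spawn function.
; After committing, a target data task supplies the hit location and actor, and the location goes to the avatar through the combat interface.
; The montage's gameplay event spawns the bolt from the weapon socket with a pitch override.
; Montage completion, blend-out, interruption, cancellation or a failed commit ends the ability on authority only.
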(event Ability|EventActivateAbility
  (bind _returnvalue (Ability|CommitAbility))
  (if _returnvalue
    (bind _datahandle (|TagetData)
      (:TargetData
        (if (Utilities|DoesObjectImplementInterface (Ability|GetAvatarActorfromActorInfo) "/Script/GAS_Game.ICombatInterface")
          (Variables|Default|SetLocation (.Location (Collision|BreakHitResult (Ability|TargetData|GetHitResultfromTargetData _datahandle))))
          (Variables|Default|SetHit%20Actor (.HitActor (Collision|BreakHitResult (Ability|TargetData|GetHitResultfromTargetData _datahandle))))
          (Class|ICombatInterface|WrapActorInterface(Message) (Ability|GetAvatarActorfromActorInfo) (Variables|Default|GetLocation))
          (|PlayMontageandWaitProxy "None" "/Game/Assets/Characters/Aura/Animations/Abilities/AM_Cast_FireBolt.AM_Cast_FireBolt" 1.0 "None" false 1.0 0.0 false
            (:then
              (Ability|Tasks|WaitGameplayEvent "(TagName=\"Event.Montage.FireBolt\")" 0 true
                (:EventReceived
                  (Class|ProjectileSpell|SpawnFireBolt (Variables|Default|GetLocation) "(TagName=\"Socket.Weapon\")" (Variables|Default|GetHit%20Actor) true 3e+01))))
            (:OnCompleted
              (Ability|HasAuthority :!label _label
                (:True
                  (Ability|EndAbility))))
            (:OnBlendOut
              (goto _label))
            (:OnInterrupted
              (goto _label))
            (:OnCancelled
              (goto _label))))))
    (else
      (Ability|HasAuthority
        (:True
          (Ability|EndAbility))))))

(event Ability|EventOnEndAbility
  (params (bWasCancelled :type Boolean)))