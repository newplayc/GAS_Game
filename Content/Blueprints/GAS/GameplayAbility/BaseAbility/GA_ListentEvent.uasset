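; GA_ListentEvent is a gameplay ability that turns gameplay events into self-applied effects for incoming experience and primary attribute points.
; On activation it starts two event waits, one for the IncomingExp meta tag and one for any tag under Attributes.Primary.
; Each received event builds a spec from that branch's effect class, passing the event's tag and magnitude as SetByCaller before applying it to the owner.
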(event Ability|EventActivateAbility
  (bind _returnvalue (Ability|GetAbilitySystemComponentfromActorInfo))
  (bind _returnvalue_2 (Ability|GetAbilitySystemComponentfromActorInfo))
  (Utilities|FlowControl|Sequence
    (:then_0
      ;[1 1 1] 添加经验
      (bind _payload (Ability|Tasks|WaitGameplayEvent "(TagName=\"Attributes.Meta.IncomingExp\")" 0)
        (:EventReceived
          (bind _returnvalue_3 (Ability|GameplayEffect|AssignTagSetbyCallerMagnitude (GameplayEffects|MakeOutgoingSpec _returnvalue_2 (Variables|Default|GetInComing%20Effect%20Class) (Math|Conversions|ToFloat(Integer) (Ability|GetAbilityLevel)) (GameplayEffects|MakeEffectContext _returnvalue_2)) (.EventTag (Utilities|Struct|BreakGameplayEventData _payload)) (.EventMagnitude (Utilities|Struct|BreakGameplayEventData _payload))))
          (GameplayEffects|ApplyGameplayEffectSpecToSelf (Ability|GetAbilitySystemComponentfromActorInfo) _returnvalue_3))))
    (:then_1
      ;[1 1 1] 添加主属性点 （力量 ---）
      (bind _payload_2 (Ability|Tasks|WaitGameplayEvent "(TagName=\"Attributes.Primary\")" 0 false false)
        (:EventReceived
          (bind _returnvalue_4 (Ability|GameplayEffect|AssignTagSetbyCallerMagnitude (GameplayEffects|MakeOutgoingSpec _returnvalue (Variables|Default|GetAttributeEffectClass) (Math|Conversions|ToFloat(Integer) (Ability|GetAbilityLevel)) (GameplayEffects|MakeEffectContext _returnvalue)) (.EventTag (Utilities|Struct|BreakGameplayEventData _payload_2)) (.EventMagnitude (Utilities|Struct|BreakGameplayEventData _payload_2))))
          (GameplayEffects|ApplyGameplayEffectSpecToSelf (Ability|GetAbilitySystemComponentfromActorInfo) _returnvalue_4))))))