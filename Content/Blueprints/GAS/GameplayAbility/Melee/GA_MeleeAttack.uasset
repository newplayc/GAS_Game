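; Gameplay ability for a melee attack, with avatar-specific data fetched through interface calls.
; On activation it passes the target's location to the avatar's warp call, then plays a random attack montage of the configured type.
; The montage's tagged gameplay event triggers a sphere overlap at its weapon socket.
; Non-friendly hits get an impact cue and server-only effect application, then a tagged cue for sound fires and the ability ends.
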(event Ability|EventActivateAbility
  (bind _returnvalue (Ability|GetAvatarActorfromActorInfo))
  (bind _returnvalue_2 (Ability|GetAvatarActorfromActorInfo))
  (bind _returnvalue_3 (Class|EnemyInterface|GetTargetActor(Message) _returnvalue))
  (Class|ICombatInterface|WrapActorInterface(Message) _returnvalue (Transformation|GetActorLocation _returnvalue_3))
  (bind _returnvalue_4 (Class|ICombatInterface|GetAttackMontage(Message) _returnvalue))
  (bind _returnvalue_5 (Class|AuraBlueprintFunctionLibrary|GetTagMontageTypewithType _returnvalue_4 (Variables|Default|GetAtt%20Type)))
  (Variables|Default|SetTagMontage (.OutItem (Utilities|Array|Random _returnvalue_5)))
  (|PlayMontageandWaitProxy "None" (.attackmontage (Variables|Default|GetTagMontage)) 1.0 "None" true 1.0 0.0 false
    (:then
      (Ability|Async|WaitGameplayEventToActor _returnvalue (.montagetag (Variables|Default|GetTagMontage)) true
        (:EventReceived
          (bind _returnvalue_6 (Class|ICombatInterface|GetWeaponSocketLocation(Message) _returnvalue (.sockettag (Variables|Default|GetTagMontage))))
          (bind _output_get (Variables|Default|SetWeaponSocketLocation _returnvalue_6))
          (bind _hitactors (Class|AuraBlueprintFunctionLibrary|GetOverlapActors _returnvalue_2 _output_get (Utilities|Array|MakeArray _returnvalue_2) 1e+02))
          (for _array_element _hitactors
            (bind _returnvalue_7 (Class|AuraBlueprintFunctionLibrary|IsFriend _array_element (Ability|GetAvatarActorfromActorInfo)))
            (if (not _returnvalue_7)
              (GameplayCue|ExecuteGameplayCueOnActor(Burst) _array_element "(TagName=\"GameplayCue.MeleeAttackEffect\")" (Ability|GameplayCue|MakeGameplayCueParameters :Location (Variables|Default|GetWeaponSocketLocation)))
              (Ability|HasAuthority
                (:True
                  (bind _returnvalue_8 (Class|AuraGameplayDamageAbility|MakeDefaultEffectParams _array_element))
                  (Class|AuraBlueprintFunctionLibrary|ApplyEffectParams _returnvalue_8)))))
          ;[1 1 1] 统一产生声音
          (GameplayCue|ExecuteGameplayCueOnActor(Burst) _array_element "(TagName=\"GameplayCue.MeleeAttackEffect\")" (Ability|GameplayCue|MakeGameplayCueParameters :AggregatedSourceTags (GameplayTags|MakeGameplayTagContainerfromArray (Utilities|Array|MakeArray (.montagetag (Variables|Default|GetTagMontage)))) :Location (Variables|Default|GetWeaponSocketLocation) :SourceObject (Ability|GetAvatarActorfromActorInfo)))
          (Ability|EndAbility))))))