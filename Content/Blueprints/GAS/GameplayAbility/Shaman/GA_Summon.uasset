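; Shaman gameplay ability that summons minions of SummonClass, expected to be BP_Demon, at shuffled spawn locations.
; Each pass bumps the avatar's summon count, plays a tagged attack montage, then waits for its gameplay event to spawn a ground effect and minion.
; After a short delay it loops until locations run out or MaxSummon is reached, then ends.
; A failed BP_Demon cast halts the loop without ending the ability.
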(event Ability|EventActivateAbility
  (Variables|Default|SetAvator (Ability|GetAvatarActorfromActorInfo))
  (bind _returnvalue (Class|ShamanSummon|GetSpawnLocations))
  (bind _output_get (Variables|Default|SetLocations _returnvalue))
  (Variables|Default|SetLength (Utilities|Array|Length _output_get))
  (Utilities|Array|Shuffle _output_get)
  (bind _returnvalue_2 (Class|ICombatInterface|GetSummonNum(Message) (Variables|Default|GetAvator) :!label _label))
  (if (and (< (Variables|Default|Getindex) (Variables|Default|GetLength)) (< _returnvalue_2 (Variables|Default|GetMaxSummon)))
    (Class|ICombatInterface|ChangeSummonNum(Message) (Variables|Default|GetAvator) 1)
    (bind _output_get_2 (Variables|Default|Setlo (Utilities|Array|Get(acopy) (Variables|Default|GetLocations) (Variables|Default|Getindex))))
    (bind _returnvalue_3 (Class|ICombatInterface|GetAttackMontage(Message) (Variables|Default|GetAvator)))
    (bind _returnvalue_4 (Class|AuraBlueprintFunctionLibrary|GetTagMontageTypewithType _returnvalue_3 (Variables|Default|GetAtt%20Type)))
    (|PlayMontageandWaitProxy "None" (.AttackMontage (Utilities|Struct|BreakTagMontage (Utilities|Array|Get(acopy) _returnvalue_4))) 1.0 "None" true 1.0 0.0 false
      (:then
        (Ability|Async|WaitGameplayEventToActor (Variables|Default|GetAvator) (.MontageTag (Utilities|Struct|BreakTagMontage (Utilities|Array|Get(acopy) _returnvalue_4))) true
          (:EventReceived
            (Niagara|SpawnSystematLocation "/Game/Assets/Effects/Combat/NS_GroundSummon.NS_GroundSummon" _output_get_2)
            (bind _returnvalue_5 (Game|SpawnActorfromClass (Variables|Default|GetSummonClass) (Math|Transform|MakeTransform _output_get_2 "0, 0, 0" "1.000000,1.000000,1.000000") "Undefined" "MultiplyWithRoot" 0 0))
            (Utilities|Casting|CastToBP_Demon _returnvalue_5)
            (Math|Integer|IncrementInt (Variables|Default|Getindex)
              (:%20%20
                (Utilities|FlowControl|Delay 0.5)
                (goto _label)))))))
    (else
      (Ability|EndAbility))))